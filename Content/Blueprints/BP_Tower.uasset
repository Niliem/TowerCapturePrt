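; Capturable tower that holds power for a Red, Blue or neutral team, with team-colored material and a selection light.
; Owned towers gain tier-based income every second; incoming power reinforces allies or drains others, turning neutral at zero and switching teams below it.
; Each power change picks the last qualifying TowerArray tier for mesh and income, then updates the widget.
; An AI attack delay, settable per team, counts down on Tick.
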(event `self.ReceiveBeginPlay`
  (`self.Update Tower Data`)
  (`KismetSystemLibrary.K2_SetTimerDelegate` (delegate `CustomEvent_0`) 1.0 true)
  (bind _asbp_tower_info (cast `/Game/Blueprints/BP_TowerInfo` (`WidgetComponent.GetUserWidgetObject` (`self.Widget`))))
  (bind _output_get (set `self.TowerUI` _asbp_tower_info))
  (`/Game/Blueprints/BP_TowerInfo.SetPowerUI` _output_get (`KismetMathLibrary.Round` (`self.CurrentPower`)))
  (`self.SetTeamColor` (`self.CurrentTeam`)))

(event `CustomEvent_0`
  (bind (_currenttowerdata_mesh _currenttowerdata_income) (break `/Game/Blueprints/STower` (`self.CurrentTowerData`)))
  (if (`|EnumInequality` (`self.CurrentTeam`) "NewEnumerator0")
    (`self.ModifyPower` _currenttowerdata_income)))

(event `self.ReceiveTick`
  (params (DeltaSeconds :type "Float (single-precision)"))
  (if (>= (`self.AIAttackDelay`) 0.0)
    (set `self.AIAttackDelay` (- (`self.AIAttackDelay`) DeltaSeconds))))

(fn `GetHalfPower`
  (returns (HalfPower :type Integer))
  (return (/ (`KismetMathLibrary.Round` (`self.CurrentPower`)) 2)))

(fn `ModifyPower`
  (params (Delta :type "Float (double-precision)"))
  (`self.SetPower` (+ Delta (`self.CurrentPower`))))

(fn `SetMesh`
  (params (NewMesh :type "StaticMesh Object Reference"))
  (`/Engine/EditorBlueprintResources/StandardMacros.IsValid` NewMesh
    (:`Is Valid`
      (`StaticMeshComponent.SetStaticMesh` (`self.TowerMesh`) NewMesh))))

(fn `SetPower`
  (params (NewPower :type "Float (double-precision)"))
  (bind _towerui (`self.TowerUI`))
  (bind _output_get (set `self.CurrentPower` NewPower))
  (`self.Update Tower Data`)
  (`/Engine/EditorBlueprintResources/StandardMacros.IsValid` _towerui
    (:`Is Valid`
      (`/Game/Blueprints/BP_TowerInfo.SetPowerUI` _towerui (`KismetMathLibrary.Round` _output_get)))))

(fn `SetSelect`
  (params (bSelect :type Boolean))
  (`SceneComponent.SetVisibility` (`self.PointLight`) bSelect false))

(fn `SetTeam`
  (params (NewTeam :type "/Game/Blueprints/ETeams Enum" :default "NewEnumerator0"))
  (bind _output_get (set `self.CurrentTeam` NewTeam))
  (`self.SetTeamColor` _output_get))

(fn `SetTeamColor`
  (params (Team :type "/Game/Blueprints/ETeams Enum" :default "NewEnumerator0"))
  (switch `/Game/Blueprints/ETeams` Team
    (:`NewEnumerator0`
      (`PrimitiveComponent.SetMaterial` (`self.TowerMesh`) 0 "/Game/Materials/MI_Base_Gray.MI_Base_Gray"))
    (:`NewEnumerator1`
      (`PrimitiveComponent.SetMaterial` (`self.TowerMesh`) 0 "/Game/Materials/MI_Base_Red.MI_Base_Red"))
    (:`NewEnumerator2`
      (`PrimitiveComponent.SetMaterial` (`self.TowerMesh`) 0 "/Game/Materials/MI_Base_Blue.MI_Base_Blue"))))

(fn `TakePower`
  (params (Power :type Integer) (Team :type "/Game/Blueprints/ETeams Enum" :default "NewEnumerator0"))
  (bind _returnvalue (`KismetMathLibrary.Conv_IntToDouble` Power))
  (if (== Team (`self.CurrentTeam`))
    (`self.ModifyPower` _returnvalue)
    (else
      (`self.ModifyPower` (* _returnvalue -1.0))
      (`/Engine/EditorBlueprintResources/StandardMacros.CompareFloat` (`self.CurrentPower`)
        (:`==`
          (`self.SetTeam` "NewEnumerator0"))
        (:`<`
          (`self.SetTeam` (`local.Team`))))
      (`self.SetPower` (`KismetMathLibrary.Abs` (`self.CurrentPower`))))))

(fn `TrySetAIDelay`
  (params (Team :type "/Game/Blueprints/ETeams Enum" :default "NewEnumerator0") (Delay :type "Float (double-precision)"))
  (if (`|EnumEquality` Team (`self.CurrentTeam`))
    (set `self.AIAttackDelay` Delay)))

(fn `Update Tower Data`
  (locals (LevelPerPower :type "Array of Float (double-precision)") (LevelIndex :type Integer))
  (for _array_element (`self.TowerArray`)
    (if (>= (`self.CurrentPower`) (`.RequarePower_8_AB52CB854932BD768604329E55524F22` (break `/Game/Blueprints/STower` _array_element)))
      (set `self.CurrentTowerData` _array_element)))
  (`self.SetMesh` (`.Mesh_2_AFA322074CE6108E953E7BAFEC693A7C` (break `/Game/Blueprints/STower` (`self.CurrentTowerData`)))))

(fn `UserConstructionScript`
  (`self.SetTeamColor` (`self.CurrentTeam`))
  (`self.Update Tower Data`))
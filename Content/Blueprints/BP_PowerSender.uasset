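; BP_PowerSender is an actor that carries an amount of power from one tower to another.
; On BeginPlay it deducts the amount from the source tower, then a timeline lerps it from its current location toward the target tower each update.
; When the timeline finishes, it hands the power and team to the target, tries to set that tower's AI delay, and destroys itself.
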(event `self.ReceiveBeginPlay`
  (`/Game/Blueprints/BP_Tower.ModifyPower` (`self.FromTower`) (* (`self.Amount`) -1.0))
  (bind (_direction _alpha) (`Timeline|Alpha`)
    (:`Update`
      (`self.K2_SetActorLocation` (`KismetMathLibrary.VLerp` (`self.K2_GetActorLocation`) (`self.K2_GetActorLocation` (`self.ToTower`)) _alpha)))
    (:`Finished`
      (`/Game/Blueprints/BP_Tower.TakePower` (`self.ToTower`) (`self.Amount`) (`self.Team`))
      (`/Game/Blueprints/BP_Tower.TrySetAIDelay` (`self.ToTower`) (`self.Team`) (`self.AIDelay`))
      (`self.K2_DestroyActor`))))

(fn `UserConstructionScript`)